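; Key pickup actor that gives the player a key.
; Any actor overlap sets HasKey on player 0's Player_BP, plays a pickup sound and destroys the key, without checking which actor overlapped.
; BeginPlay stores a random Z offset and the placed height, but never moves the key.
; A sine-based vertical motion is left disconnected, and Tick does nothing.
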(event `self.ReceiveBeginPlay`
  (set `self.InitialZ` (`KismetMathLibrary.RandomFloatInRange` -20.0 20.0))
  (set `self.InitialLocation` (`KismetMathLibrary.MakeVector` 0.0 0.0 (`self.InitialZ`)))
  (bind _output_get (set `self.PlacedLocation` (`self.K2_GetActorLocation`)))
  (set `self.BaseZLocation` (.z _output_get)))

(event `self.ReceiveActorBeginOverlap`
  (params (OtherActor :type "Actor Object Reference"))
  (bind _asplayer_bp (cast `/Game/_Game/Blueprints/Actors/PlayerCharacter/Player_BP` (`GameplayStatics.GetPlayerCharacter` 0)))
  (set `/Game/_Game/Blueprints/Actors/PlayerCharacter/Player_BP.bHasKey` true _asplayer_bp)
  (`GameplayStatics.PlaySound2D` "/Game/_Game/Sound/SoundEffects/KeyPickUp_Cue.KeyPickUp_Cue" 1.0 1.0 0.0 null null)
  (`self.K2_DestroyActor`))

(event `self.ReceiveTick`
  (params (DeltaSeconds :type "Float (single-precision)")))

(fn `UserConstructionScript`)