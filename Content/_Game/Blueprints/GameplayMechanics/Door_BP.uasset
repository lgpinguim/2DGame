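; Door Blueprint for a Paper2D game that plays its flipbook animation when the player overlaps it while holding a key.
; On overlap it casts the player character to Player_BP and checks HasKey, then a DoOnce plays the flipbook from the start without looping.
; The construction script pins the door to a fixed Y depth while keeping its X and Z position.
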(event `self.ReceiveActorBeginOverlap`
  (params (OtherActor :type "Actor Object Reference"))
  (if (== OtherActor (`GameplayStatics.GetPlayerCharacter` 0))
    (bind _asplayer_bp (cast `/Game/_Game/Blueprints/Actors/PlayerCharacter/Player_BP` (`GameplayStatics.GetPlayerCharacter` 0)))
    (if (`/Game/_Game/Blueprints/Actors/PlayerCharacter/Player_BP.bHasKey` _asplayer_bp)
      (`/Engine/EditorBlueprintResources/StandardMacros.DoOnce` false
        (:`Completed`
          (`PaperFlipbookComponent.PlayFromStart` (`self.PaperFlipbook`))
          (`PaperFlipbookComponent.SetLooping` (`self.PaperFlipbook`) false))))))

(fn `UserConstructionScript`
  (bind (_returnvalue_x _returnvalue_y _returnvalue_z) (`KismetMathLibrary.BreakVector` (`self.K2_GetActorLocation`)))
  (`self.K2_SetActorLocation` (`KismetMathLibrary.MakeVector` _returnvalue_x -0.3 _returnvalue_z)))