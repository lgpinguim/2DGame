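; GoldCoin_BP is a gold coin pickup that the player collects by overlapping it.
; On overlap with the player character, it adds one to Gold on Player_BP, plays a 2D pickup sound and destroys itself.
; The construction script keeps the coin's X and Z but leaves Y unset, which appears to snap it onto the Y=0 plane.
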(event `self.ReceiveActorBeginOverlap`
  (params (OtherActor :type "Actor Object Reference"))
  (if (== OtherActor (`GameplayStatics.GetPlayerCharacter` 0))
    (bind _asplayer_bp (cast `/Game/_Game/Blueprints/Actors/PlayerCharacter/Player_BP` (`GameplayStatics.GetPlayerCharacter` 0)))
    (set `/Game/_Game/Blueprints/Actors/PlayerCharacter/Player_BP.Gold` (+ (`/Game/_Game/Blueprints/Actors/PlayerCharacter/Player_BP.Gold` _asplayer_bp) 1) _asplayer_bp)
    (`GameplayStatics.PlaySound2D` "/Game/_Game/Sound/SoundEffects/CoinPickUp_Cue.CoinPickUp_Cue" 1.0 1.0 0.0 null null)
    (`self.K2_DestroyActor`)))

(fn `UserConstructionScript`
  (bind (_returnvalue_x _returnvalue_y _returnvalue_z) (`KismetMathLibrary.BreakVector` (`self.K2_GetActorLocation`)))
  (`self.K2_SetActorLocation` (`KismetMathLibrary.MakeVector` _returnvalue_x 0.0 _returnvalue_z)))