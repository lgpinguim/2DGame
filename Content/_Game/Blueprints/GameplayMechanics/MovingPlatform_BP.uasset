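; MovingPlatform_BP is a platform actor that shuttles continuously back and forth between its starting position and a target point.
; BeginPlay caches the start and converts TargetLocation, treated as an unrotated offset from the actor's position, into a world-space target.
; Tick moves it at constant Speed without sweep, swapping endpoints once travelled distance reaches the journey length.
; The construction script keeps X and Z but sets Y to its unconnected default, apparently zero.
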(event `self.ReceiveBeginPlay`
  (set `self.LocalStartLocation` (`self.K2_GetActorLocation`))
  (set `self.LocalTargetLocation` (`KismetMathLibrary.TransformLocation` (`KismetMathLibrary.Conv_VectorToTransform` (`self.K2_GetActorLocation`)) (`self.TargetLocation`))))

(event `self.ReceiveTick`
  (params (DeltaSeconds :type "Float (single-precision)"))
  (set `self.Location` (`self.K2_GetActorLocation`))
  (set `self.JourneyLength` (`KismetMathLibrary.VSize` (- (`self.LocalTargetLocation`) (`self.LocalStartLocation`))))
  (set `self.JourneyTravelled` (`KismetMathLibrary.VSize` (- (`self.Location`) (`self.LocalStartLocation`))))
  (if (>= (`self.JourneyTravelled`) (`self.JourneyLength`))
    (set `self.Swap` (`self.LocalStartLocation`))
    (set `self.LocalStartLocation` (`self.LocalTargetLocation`))
    (set `self.LocalTargetLocation` (`self.Swap`))
    (set `self.Direction` (`KismetMathLibrary.Normal` (- (`self.LocalTargetLocation`) (`self.LocalStartLocation`))))
    (`self.K2_SetActorLocation` (+ (`self.K2_GetActorLocation`) (* (`self.Direction`) (* DeltaSeconds (`self.Speed`)))))
    (else
      (set `self.Direction` (`KismetMathLibrary.Normal` (- (`self.LocalTargetLocation`) (`self.LocalStartLocation`))))
      (`self.K2_SetActorLocation` (+ (`self.K2_GetActorLocation`) (* (`self.Direction`) (* DeltaSeconds (`self.Speed`))))))))

(fn `UserConstructionScript`
  (bind (_returnvalue_x _returnvalue_y _returnvalue_z) (`KismetMathLibrary.BreakVector` (`self.K2_GetActorLocation`)))
  (`self.K2_SetActorLocation` (`KismetMathLibrary.MakeVector` _returnvalue_x 0.0 _returnvalue_z)))