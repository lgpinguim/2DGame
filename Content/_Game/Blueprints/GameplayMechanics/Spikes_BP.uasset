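; Spike hazard for a side-scroller that damages the player on touch and knocks them back.
; Box overlap with a living player calls DamagePlayer, which cuts health, plays impact and pain sounds, and launches the character upward and horizontally using the hit normal.
; It also starts a looping timer on DamagePlayer by name, cleared when overlap ends.
; The construction script snaps the actor to Y zero, keeping X and Z.
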(event `self.BoxCollision.OnComponentBeginOverlap`
  (params (OverlappedComponent :type "PrimitiveComponent Object Reference") (OtherActor :type "Actor Object Reference") (OtherComp :type "PrimitiveComponent Object Reference") (OtherBodyIndex :type Integer) (bFromSweep :type Boolean) (SweepResult :type "HitResult Structure (by ref)"))
  (bind _asplayer_bp (cast `/Game/_Game/Blueprints/Actors/PlayerCharacter/Player_BP` OtherActor))
  (if (not (`/Game/_Game/Blueprints/Actors/PlayerCharacter/Player_BP.IsDead` _asplayer_bp))
    (`self.DamagePlayer` SweepResult)
    (bind _returnvalue (`KismetSystemLibrary.K2_SetTimer` null "DamagePlayer" 0.75 true))))

(event `self.ReceiveActorEndOverlap`
  (params (OtherActor :type "Actor Object Reference"))
  (`KismetSystemLibrary.K2_ClearAndInvalidateTimerHandle` (stale `self.BoxCollision.OnComponentBeginOverlap` _returnvalue)))

(fn `DamagePlayer`
  (params (NewParam :type "HitResult Structure"))
  (bind _asplayer_bp (cast `/Game/_Game/Blueprints/Actors/PlayerCharacter/Player_BP` (`GameplayStatics.GetPlayerCharacter` 0)))
  (set `self.As 2DSide Scroller Character` _asplayer_bp)
  (bind _health (`/Game/_Game/Blueprints/Actors/PlayerCharacter/Player_BP.Health` _asplayer_bp))
  (if (> _health 0)
    (set `/Game/_Game/Blueprints/Actors/PlayerCharacter/Player_BP.Health` (- _health 10) _asplayer_bp)
    (`GameplayStatics.PlaySound2D` "/Game/_Game/Sound/SoundEffects/Metal_bang_3_Cue.Metal_bang_3_Cue" 1.0 1.0 0.0 null null)
    (`GameplayStatics.PlaySound2D` "/Game/_Game/Sound/CharacterSound/voice_male_grunt_pain_06_Cue.voice_male_grunt_pain_06_Cue" 1.0 1.0 0.0 null null)
    (`Character.LaunchCharacter` _asplayer_bp (`KismetMathLibrary.MakeVector` (* (.x (`.Normal` (`GameplayStatics.BreakHitResult` NewParam))) -400.0) 0.0 600.0) true true)))

(fn `UserConstructionScript`
  (bind (_returnvalue_x _returnvalue_y _returnvalue_z) (`KismetMathLibrary.BreakVector` (`self.K2_GetActorLocation`)))
  (`self.K2_SetActorLocation` (`KismetMathLibrary.MakeVector` _returnvalue_x 0.0 _returnvalue_z)))