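; Player character Blueprint for a 2D side-scroller knight, handling movement, jumping, a melee-button attack and death.
; Tick picks the flipbook from falling, attack and velocity state, turns the controller to face travel direction, and flags death when Health runs out.
; Attack locks input, then spawns Projectile_BP after a delay at a fixed +X offset.
; Death plays animation and sound, then reloads the example map; the staged-attack animation function is never called here.
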(event `UpdateAnimation`
  (bind _bisattacking (`self.bIsAttacking`))
  ;[1 1 1] Handle Animation
  (if (`self.IsDead`)
    (`/Engine/EditorBlueprintResources/StandardMacros.DoOnce` false
      (:`Completed`
        (`self.Play Death Animation`)
        (`KismetSystemLibrary.Delay` 5.0)
        (`GameplayStatics.OpenLevel` "2DSideScrollerExampleMap")))
    (elif (`NavMovementComponent.IsFalling` (`self.CharacterMovement`))
      (`PaperFlipbookComponent.SetFlipbook` (`self.Sprite`) "/Game/_Game/Blueprints/Actors/PlayerCharacter/Jump/KnightJumpAndFall_FlipBook.KnightJumpAndFall_FlipBook")
      (else
        (`PaperFlipbookComponent.SetFlipbook` (`self.Sprite`) (select `bool` _bisattacking :`false` (select `bool` (> (`KismetMathLibrary.VSize` (`self.GetVelocity`)) 0.0) :`false` "/Game/_Game/Blueprints/Actors/PlayerCharacter/Idle/KnightIdle_FlipBook.KnightIdle_FlipBook" :`true` "/Game/_Game/Blueprints/Actors/PlayerCharacter/Run/KnightRun_FlipBook.KnightRun_FlipBook" :!type "PaperFlipbook Object Reference") :`true` (select `bool` _bisattacking :`false` "/Game/_Game/Blueprints/Actors/PlayerCharacter/Idle/KnightIdle_FlipBook.KnightIdle_FlipBook" :`true` "/Game/_Game/Blueprints/Actors/PlayerCharacter/Attack/KnightAttack1_Flipbook.KnightAttack1_Flipbook" :!type "PaperFlipbook Object Reference")))))))

(event `self.ReceiveBeginPlay`
  (`ActorComponent.SetIsReplicated` (`self.Sprite`) true))

(event `InputAction|MeleeAttack`
  (params (Key :type "Key Structure"))
  ;[1 1 1] Handle Animation
  (:`Pressed`
    (`PaperFlipbookComponent.SetFlipbook` (`self.Sprite`) "/Game/_Game/Blueprints/Actors/PlayerCharacter/Attack/KnightAttack1_Flipbook.KnightAttack1_Flipbook"))
  (:`Released`
    (`PaperFlipbookComponent.SetFlipbook` (`self.Sprite`) "/Game/_Game/Blueprints/Actors/PlayerCharacter/Idle/KnightIdle_FlipBook.KnightIdle_FlipBook")))

(event `InputAction|MeleeAttack`
  (params (Key :type "Key Structure"))
  (bind _returnvalue (`self.GetTransform`))
  ;[1 1 1] Handle Animation
  (:`Pressed`
    (`/Engine/EditorBlueprintResources/StandardMacros.DoOnce` false :!label _label
      (:`Completed`
        (`self.DisableInput` null)
        (set `self.bIsAttacking` true)
        (`KismetSystemLibrary.Delay` 0.9)
        (`|SpawnActorFromClass` "/Game/_Game/Blueprints/Projectile_BP.Projectile_BP_C" (`KismetMathLibrary.MakeTransform` (`KismetMathLibrary.MakeVector` (+ (.x (.location _returnvalue)) 160.0) 0.0 (+ (.z (.location _returnvalue)) 1.0)) (.rotation _returnvalue)) "Undefined" "OverrideRootScale" null null)
        (set `self.bIsAttacking` false)
        (`self.EnableInput` null)
        (goto _label :!via `Reset`)))))

(event `self.ReceiveTick`
  (params (DeltaSeconds :type "Float (single-precision)"))
  (bind _returnvalue (`self.GetController`))
  (bind _returnvalue_2 (`self.GetController`))
  ;[1 1 1] Tick - Updates animation
  (`|ExecutionSequence`
    (:`then_0`
      (`self.UpdateAnimation`)
      (`/Engine/EditorBlueprintResources/StandardMacros.CompareFloat` (.x (`MovementComponent.Velocity` (`self.GetMovementComponent`)))
        (:`>`
          (`/Engine/EditorBlueprintResources/StandardMacros.IsValid` _returnvalue_2 :!label _label_2
            (:`Is Valid`
              (`Controller.SetControlRotation` _returnvalue_2 (`KismetMathLibrary.MakeRotator` 0.0)))))
        (:`==`
          (if (`self.bisMovingRight`)
            (goto _label_2)
            (else
              (`/Engine/EditorBlueprintResources/StandardMacros.IsValid` _returnvalue :!label _label_3
                (:`Is Valid`
                  (`Controller.SetControlRotation` _returnvalue (`KismetMathLibrary.MakeRotator` 0.0 0.0 180.0)))))))
        (:`<`
          (goto _label_3))))
    (:`then_1`
      (if (<= (`self.Health`) 0)
        (set `self.IsDead` true)))))

(event `InputAxis|MoveRight`
  (params (AxisValue :type "Float (single-precision)"))
  ;[1 1 1] Handle movement
  (if (> AxisValue 0.0)
    (set `self.bisMovingRight` true)
    (elif (< AxisValue 0.0)
      (set `self.bisMovingRight` false)))
  (`self.AddMovementInput` (1.0 0.0 0.0) AxisValue))

(event `InputAction|Jump`
  (params (Key :type "Key Structure"))
  ;[1 1 1] Handle Jump
  (:`Pressed`
    (`self.Jump` :!label _label_4)
    (if (not (`NavMovementComponent.IsFalling` (`self.CharacterMovement`)))
      (`GameplayStatics.SpawnSoundAtLocation` "/Game/_Game/Sound/CharacterSound/Jump_Cue.Jump_Cue" (`self.K2_GetActorLocation`) (struct) 1.0 1.0 0.0 null null)))
  (:`Released`
    (`self.StopJumping` :!label _label_5)))

(event `InputTouch`
  (params (Location :type "Vector Structure") (FingerIndex :type "ETouchIndex Enum"))
  ;[1 1 1] Handle Jump
  (:`Pressed`
    (goto _label_4))
  (:`Released`
    (goto _label_5)))

(fn `Play Attack Animation`
  (params (AttackStage :type Integer))
  (`PaperFlipbookComponent.SetLooping` (`self.Sprite`) false)
  (switch `int` AttackStage
    (:`Default`
      (set `self.AttackStage` 0)
      (`PaperFlipbookComponent.SetFlipbook` (`self.Sprite`) "/Game/_Game/Blueprints/Actors/PlayerCharacter/Idle/KnightIdle_FlipBook.KnightIdle_FlipBook"))
    (:`1`
      (bind _returnvalue (`PaperFlipbookComponent.SetFlipbook` (`self.Sprite`) "/Game/_Game/Blueprints/Actors/PlayerCharacter/Attack/KnightAttack1_Flipbook.KnightAttack1_Flipbook"))
      (set `self.IsPlayingAttackAnimation` (or _returnvalue (stale _returnvalue_2) (stale _returnvalue_3)) :!label _label)
      (`GameplayStatics.SpawnSound2D` "/Game/_Game/Sound/CharacterSound/Attack_Cue.Attack_Cue" 1.0 1.0 0.0 null))
    (:`2`
      (bind _returnvalue_2 (`PaperFlipbookComponent.SetFlipbook` (`self.Sprite`) "/Game/_Game/Blueprints/Actors/PlayerCharacter/Attack/KnightAttack2_Flipbook.KnightAttack2_Flipbook"))
      (goto _label))
    (:`3`
      (bind _returnvalue_3 (`PaperFlipbookComponent.SetFlipbook` (`self.Sprite`) "/Game/_Game/Blueprints/Actors/PlayerCharacter/Attack/KnightAttack3_Flipbook.KnightAttack3_Flipbook"))
      (goto _label))))

(fn `Play Death Animation`
  (`self.DisableInput` null)
  (`PaperFlipbookComponent.SetFlipbook` (`self.Sprite`) "/Game/_Game/Blueprints/Actors/PlayerCharacter/Death/KnightDeath_Flipbook.KnightDeath_Flipbook")
  (`PaperFlipbookComponent.SetLooping` (`self.Sprite`) false)
  (`GameplayStatics.SpawnSound2D` "/Game/HumanVocalizations/HumanMaleB/Cues/voice_male_b_death_low_01_Cue.voice_male_b_death_low_01_Cue" 1.0 1.0 0.0 null))

(fn `UserConstructionScript`
  (bind (_returnvalue_x _returnvalue_y _returnvalue_z) (`KismetMathLibrary.BreakVector` (`self.K2_GetActorLocation`)))
  (`self.K2_SetActorLocation` (`KismetMathLibrary.MakeVector` _returnvalue_x 0.0 _returnvalue_z)))