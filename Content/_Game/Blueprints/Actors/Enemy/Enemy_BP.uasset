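; Skeleton enemy for a Paper2D game that patrols between PointA and PointB, hurting and knocking back the player on capsule overlap.
; Construction feeds both points to InterpToMovement, whose reverse event flips the sprite.
; Tick selects idle, walk or hit flipbooks, clears the hit flag after a delay, and polls Health.
; At zero Health, movement and collision stop, then the death flipbook and sound play once.
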(event `self.InterpToMovement.OnInterpToReverse`
  (params (ImpactResult :type "HitResult Structure (by ref)") (Time :type "Float (single-precision)"))
  (bind _paperflipbook (`self.PaperFlipbook`))
  (if (not (`self.IsDead`))
    (`/Engine/EditorBlueprintResources/StandardMacros.FlipFlop`
      (:`A`
        (`SceneComponent.K2_SetWorldRotation` :`self` _paperflipbook))
      (:`B`
        (`SceneComponent.K2_SetWorldRotation` _paperflipbook (struct :`Yaw` 180.0) false false)))))

(event `UpdateAnimation`
  (bind _isdead (`self.IsDead`))
  (if (`self.IsDead`)
    (`/Engine/EditorBlueprintResources/StandardMacros.DoOnce` false
      (:`Completed`
        (`self.Play Death Animation`)))
    (else
      (`PaperFlipbookComponent.SetFlipbook` (`self.PaperFlipbook`) (select `bool` (`self.IsTakingDamage`) :`false` (select `bool` _isdead :`false` (select `bool` (> (`KismetMathLibrary.VSize` (`MovementComponent.Velocity` (`self.InterpToMovement`))) 0.0) :`false` "/Game/_Game/Blueprints/Actors/Enemy/Idle/Skeleton_Idle_Flipbook.Skeleton_Idle_Flipbook" :`true` "/Game/_Game/Blueprints/Actors/Enemy/Walk/Skeleton_Walk_Flipbook.Skeleton_Walk_Flipbook" :!type "PaperFlipbook Object Reference") :`true` (select `bool` _isdead :`false` "/Game/_Game/Blueprints/Actors/Enemy/Walk/Skeleton_Walk_Flipbook.Skeleton_Walk_Flipbook" :`true` "/Game/_Game/Blueprints/Actors/Enemy/Death/Skeleton_Dead_flipbook.Skeleton_Dead_flipbook" :!type "PaperFlipbook Object Reference")) :`true` "/Game/_Game/Blueprints/Actors/Enemy/Hit/Skeleton_Hit_Flipbook.Skeleton_Hit_Flipbook")))))

(event `self.ReceiveTick`
  (params (DeltaSeconds :type "Float (single-precision)"))
  (bind _interptomovement (`self.InterpToMovement`))
  (`|ExecutionSequence`
    (:`then_0`
      (`self.UpdateAnimation`))
    (:`then_1`
      (`self.PlayDeath` _interptomovement _interptomovement))
    (:`then_2`
      (if (`self.IsTakingDamage`)
        (`KismetSystemLibrary.Delay` 0.6)
        (set `self.IsTakingDamage` false)))))

(event `self.Capsule.OnComponentBeginOverlap`
  (params (OverlappedComponent :type "PrimitiveComponent Object Reference") (OtherActor :type "Actor Object Reference") (OtherComp :type "PrimitiveComponent Object Reference") (OtherBodyIndex :type Integer) (bFromSweep :type Boolean) (SweepResult :type "HitResult Structure (by ref)"))
  (if (not (`self.IsDead`))
    (bind _asplayer_bp (cast `/Game/_Game/Blueprints/Actors/PlayerCharacter/Player_BP` OtherActor))
    (set `/Game/_Game/Blueprints/Actors/PlayerCharacter/Player_BP.Health` (- (`/Game/_Game/Blueprints/Actors/PlayerCharacter/Player_BP.Health` _asplayer_bp) 10) _asplayer_bp)
    (if (not (`/Game/_Game/Blueprints/Actors/PlayerCharacter/Player_BP.IsDead` _asplayer_bp))
      (`Character.LaunchCharacter` _asplayer_bp (`KismetMathLibrary.MakeVector` (* (.x (`.Normal` (`GameplayStatics.BreakHitResult` SweepResult))) -400.0) 0.0 600.0) true true)
      (`GameplayStatics.SpawnSound2D` "/Game/_Game/Sound/CharacterSound/voice_male_grunt_pain_06_Cue.voice_male_grunt_pain_06_Cue" 1.0 1.0 0.0 null))))

(fn `Interp Sprite Rotate`
  (bind _paperflipbook (`self.PaperFlipbook`))
  (if (not (`self.IsDead`))
    (`/Engine/EditorBlueprintResources/StandardMacros.FlipFlop`
      (:`A`
        (`SceneComponent.K2_SetWorldRotation` :`self` _paperflipbook))
      (:`B`
        (`SceneComponent.K2_SetWorldRotation` _paperflipbook (struct :`Yaw` 180.0) false false)))))

(fn `Play Death Animation`
  (bind _paperflipbook (`self.PaperFlipbook`))
  (`PaperFlipbookComponent.SetFlipbook` _paperflipbook "/Game/_Game/Blueprints/Actors/Enemy/Death/Skeleton_Dead_flipbook.Skeleton_Dead_flipbook")
  (`PaperFlipbookComponent.SetLooping` _paperflipbook false)
  (`GameplayStatics.SpawnSound2D` "/Engine/EditorSounds/GamePreview/EjectFromPlayer_Cue.EjectFromPlayer_Cue" 1.0 1.0 0.0 null))

(fn `PlayDeath`
  (params (self2 :type "MovementComponent Object Reference") (self3 :type "MovementComponent Object Reference"))
  (if (<= (`KismetMathLibrary.FTrunc` (`self.Health`)) 0)
    (`/Engine/EditorBlueprintResources/StandardMacros.DoOnce` false
      (:`Completed`
        (set `self.IsDead` true)
        (set `MovementComponent.Velocity` (0.0 0.0 0.0) self2)
        (`self.SetActorEnableCollision` false)
        (`MovementComponent.StopMovementImmediately` self3)))))

(fn `UserConstructionScript`
  (set `InterpToMovementComponent.ControlPoints` (`|MakeArray` (make `InterpControlPoint` (`self.PointA`)) (make `InterpControlPoint` (`self.PointB`))) (`self.InterpToMovement`)))